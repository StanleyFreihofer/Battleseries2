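; BP_Vehicle_Base2 is a data-driven base vehicle that characters can hover over and interact with to enter.
; Its construction script builds the mesh from the DT_Vehicles row for its VehicleID.
; The interaction interface shows a WB_Interact widget, supplies the vehicle's name and icon, and calls EnterVehicle.
; Landing-gear logic toggles on physics simulation, swapping to a hardcoded F-15 physics asset when raised; turret control is an empty stub.
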(event EventBeginPlay
  (|CallParentFunction))

(event EventBPIFHoverInteraction
  (params (Hovering? :type Boolean))
  (bind _interactionwidgetcomponent (Variables|Default|GetInteractionWidgetComponent))
  (if Hovering?
    (bind _aswb_interact (Utilities|Casting|CastToWB_Interact (UserInterface|GetWidget _interactionwidgetcomponent)))
    (Default|UpdateInfo _aswb_interact self)
    (Rendering|SetVisibility _interactionwidgetcomponent true false)
    (else
      (Rendering|SetVisibility _interactionwidgetcomponent false false))))

(event EventBPIInteract
  (params (Character%20Interacting :type Character%20Base%20Object%20Reference))
  (Class|VehicleBase|EnterVehicle Character%20Interacting)
  (Rendering|SetVisibility (Variables|Default|GetInteractionWidgetComponent) false false))

(event Game|Damage|EventAnyDamage
  (params (Damage :type Float%20%28single-precision%29) (DamageType :type Damage%20Type%20Object%20Reference) (InstigatedBy :type Controller%20Object%20Reference) (DamageCauser :type Actor%20Object%20Reference)))

(event EventTick
  (params (DeltaSeconds :type Float%20%28single-precision%29))
  (|CallParentFunction DeltaSeconds))

(fn ConstructionScript
  ;[0.15 0.15 0.15 0.5] used for preview purposes?
  (Class|VehicleBase|InitVehicleMesh (Utilities|ResolveSoftReference (.Vehicle_Mesh (Utilities|Struct|BreakVehicleData (CallFunction|FunctGetVehicleData))))))

(fn FunctGetVehicleData
  (bind _returnvalue (Utilities|GetDataTableRow "/Game/__SFContent/Vehicles/Data/DT_Vehicles.DT_Vehicles" (.vehicleid (Variables|Default|GetVehicleStartingData)))
    (:then
      (return _returnvalue))))

(fn FunctControlTurret
  (params (Input%20Axis :type Vector%202D%20Structure) (SeatIndex :type Integer))
  (if (.TurretMeshIsSeparateWeaponMesh (Utilities|Struct|BreakTurretData (Utilities|Array|Get(acopy) (.Turrets (Utilities|Struct|BreakVehicleData (CallFunction|FunctGetVehicleData))))))
    _))

(fn FunctUpdateLandingGear
  (bind _vehiclemeshcomponent (Variables|Default|GetVehicleMeshComponent))
  (bind _in_bone_name (Variables|Default|GetIn%20Bone%20Name))
  (if (Variables|Default|GetLandingGearDown?)
    ;[0.15 0.15 0.15 0.5] Landing Gear Down True (landing)
    (Class|SkeletalMeshComponent|SetAllBodiesBelowSimulatePhysics _vehiclemeshcomponent _in_bone_name true true)
    (else
      ;[0.15 0.15 0.15 0.5] Landing Gear Up (should be flying)
      (Components|SkinnedMesh|SetPhysicsAsset (Variables|Default|GetVehicleMeshComponent) "/Game/VigilanteContent/Vehicles/West_Fighter_F15E/PHYS_West_Fighter_F15E3.PHYS_West_Fighter_F15E3" true)
      (Class|SkeletalMeshComponent|SetAllBodiesBelowSimulatePhysics _vehiclemeshcomponent _in_bone_name true true))))

(fn BPIFGetActionType
  (return "NewEnumerator1"))

(fn BPIFGetInteractObjectInfo
  (bind _returnvalue (Subsystems|GetBPDataManagerSubsystem))
  (bind _vehiclestartingdata (Variables|Default|GetVehicleStartingData))
  (bind _returnvalue_2 (Class|DataManagerSubsystem|GetVehicleDataRowCopy _returnvalue (.vehicleid _vehiclestartingdata)))
  (bind (_vehicle_displayname _movement_type _vehicle_type _vehicleicon) (Utilities|Struct|BreakVehicleData _returnvalue_2))
  (return (Utilities|Text|ToText(Name) _vehicle_displayname) _vehicleicon))

(fn BPIFGetInteractType
  (return "NewEnumerator1"))
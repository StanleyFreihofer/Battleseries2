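; Editor-tool vehicle actor that previews a vehicle's mesh and seat setup from the vehicle data table.
; The construction script looks up the VehicleID row, blocking-loads its skeletal mesh, then configures the seat child actors.
; Each BP_Seat_Editor is stored in EditorSeats by SeatIndex and marked active only if that index is within the row's seat count.
; Weapon preview and older seat-spawning logic remain as disconnected nodes.
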(event EventBeginPlay)

(event Collision|EventActorBeginOverlap
  (params (OtherActor :type Actor%20Object%20Reference)))

(event EventTick
  (params (DeltaSeconds :type Float%20%28single-precision%29)))

(fn ConstructionScript
  (CallFunction|FunctLoadVehicleMeshinEditor)
  (CallFunction|FunctConfigureSeats))

(fn FunctLoadVehicleMeshinEditor
  (bind _returnvalue (Utilities|LoadAssetBlocking (.Vehicle_Mesh (Utilities|Struct|BreakVehicleData (CallFunction|FunctGetVehicleData)))))
  (bind _asskeletal_mesh (Utilities|Casting|CastToSkeletalMesh _returnvalue))
  (Components|SkeletalMesh|SetSkeletalMeshAsset (Variables|Default|GetVehicle%20Mesh) _asskeletal_mesh))

(fn FunctGetVehicleData
  (bind _returnvalue (Utilities|GetDataTableRow (Variables|Default|GetVehicle%20DT) (Variables|Default|GetVehicleID))
    (:then
      (return _returnvalue))))

(fn FunctConfigureSeats
  (Utilities|FlowControl|Sequence
    (:then_0
      (bind _output_get (Variables|Default|Set#%20of%20Seats (Utilities|Array|Length (.Seats (Utilities|Struct|BreakVehicleData (CallFunction|FunctGetVehicleData))))))
      (Development|PrintString (Utilities|String|ToString(Integer) _output_get)))
    (:then_1
      (for _array_element (Actor|GetComponentsByClass "/Script/Engine.ChildActorComponent")
        (bind _asbp_seat_editor (Utilities|Casting|CastToBP_Seat_Editor (Variables|/Script/Engine.ChildActorComponent|GetChildActor _array_element)))
        (bind _output_get_2 (LocalVariables|SetSeat _asbp_seat_editor))
        (bind _output_get_3 (LocalVariables|SetSeat%20Index (Variables|/Game/__SFContent/EditorTools/BP_Seat_Editor.BP_Seat_Editor_C|GetSeat%20Index _output_get_2)))
        (Utilities|Array|SetArrayElem (Variables|Default|GetEditorSeats) _output_get_3 _output_get_2)
        (if (< (LocalVariables|GetSeat%20Index) (Variables|Default|Get#%20of%20Seats))
          (Variables|/Game/__SFContent/EditorTools/BP_Seat_Editor.BP_Seat_Editor_C|SetisActive (LocalVariables|GetSeat) true)
          (Development|PrintString (Utilities|String|ToString(Text) (Utilities|Text|FormatText "Seat Indexx {A}" (LocalVariables|GetSeat%20Index))))
          (else
            (Variables|/Game/__SFContent/EditorTools/BP_Seat_Editor.BP_Seat_Editor_C|SetisActive (LocalVariables|GetSeat) false)))))))
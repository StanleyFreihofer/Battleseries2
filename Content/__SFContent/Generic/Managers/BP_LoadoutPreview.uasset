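; BP_LoadoutPreview is a manager actor with a debug camera toggle for the loadout preview stage and a fade-and-teleport trigger.
; Debug key 8 alternates player 0's view target between the item and loadout cameras held in PreviewStageState.
; When a BP_Char_Base2 overlaps the Box, player 0's screen fades out, then a timer moves that character to the Scene component's transform and fades back in.
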(event OnComponentBeginOverlap(Box)
  (params (OverlappedComponent :type Primitive%20Component%20Object%20Reference) (OtherActor :type Actor%20Object%20Reference) (OtherComp :type Primitive%20Component%20Object%20Reference) (OtherBodyIndex :type Integer) (bFromSweep :type Boolean) (SweepResult :type Hit%20Result%20Structure%20%28by%20ref%29))
  (bind _asbp_char_base_2 (Utilities|Casting|CastToBP_Char_Base2 OtherActor))
  (Variables|Default|SetAs%20BP%20Char%20Base%202 _asbp_char_base_2)
  (CameraFades|StartCameraFade :self (Variables|/Script/Engine.PlayerController|GetPlayerCameraManager (Game|GetPlayerController 0)) :ToAlpha 1.0 :Duration 2.0 :bHoldWhenFinished true)
  (Utilities|Time|SetTimerbyEvent (delegate Custom|CustomEvent) 2.0))

(event Custom|CustomEvent
  (Transformation|SetActorTransform (Variables|Default|GetAs%20BP%20Char%20Base%202) (Transformation|GetWorldTransform (Variables|Default|GetScene)))
  (CameraFades|StartCameraFade :self (Variables|/Script/Engine.PlayerController|GetPlayerCameraManager (Game|GetPlayerController 0)) :FromAlpha 1.0 :Duration 2.0))

(event EventBeginPlay
  (|CallParentFunction))

(event EventTick
  (params (DeltaSeconds :type Float%20%28single-precision%29)))

(event Input|KeyboardEvents|DebugKey8
  (params (Key :type Key%20Structure :default "None") (ActionValue :type Input%20Action%20Value%20Structure))
  (bind _returnvalue (Game|GetPlayerController 0))
  (bind _previewstagestate (Variables|Default|GetPreviewStageState))
  (bind (_currentstagemode _currentvehicle _previewgun_attachmentstate _rotateobject _loadoutcam _itemcam) (Utilities|Struct|BreakPreviewState _previewstagestate))
  (:Pressed
    (Utilities|FlowControl|FlipFlop
      (:A
        (Game|Player|SetViewTargetwithBlend _returnvalue _itemcam 0.0 "VTBlend_Linear" 0.0 false))
      (:B
        (Game|Player|SetViewTargetwithBlend _returnvalue _loadoutcam 0.0 "VTBlend_Linear" 0.0 false)))))

(fn ConstructionScript)
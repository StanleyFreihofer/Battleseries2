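; Base character Blueprint that adds the default Enhanced Input mapping and detects interactable actors the player looks at.
; While possessed, Tick runs a short debug-drawn sphere trace from the first-person camera, avoiding head socket wobble.
; A first hit implementing BPI_Interact gets a hover message and interact-type query; losing it clears the hover.
; A vehicle-status function toggles collision and attaches or detaches the character from the vehicle.
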(event EventBeginPlay
  (bind _asplayer_controller (Utilities|Casting|CastToPlayerController (Pawn|GetController)))
  (Input|AddMappingContext (PlayerController|LocalPlayerSubsystems|GetEnhancedInputLocalPlayerSubsystem _asplayer_controller) "/Game/__SFContent/Inputs/IMC/IMC_Default.IMC_Default" 0 "(bIgnoreAllPressedKeysUntilRelease=True,bForceImmediately=False,bNotifyUserSettings=False)"))

(event EventTick
  (params (DeltaSeconds :type Float%20%28single-precision%29))
  ;[0.15 0.15 0.15 0.5] only do this if this character is possessed
  (Utilities|IsValid (Pawn|GetController)
    (:Is%20Valid
      (bind _outhits (CallFunction|FunctRaycast (Transformation|GetWorldTransform (Variables|Default|Get1PCamera))))
      (if (> (Utilities|Array|Length _outhits) 0)
        (if (Utilities|DoesObjectImplementInterface (.HitActor (Collision|BreakHitResult (Utilities|Array|Get(acopy) _outhits))) "/Game/__SFContent/Generic/Utilities/Interfaces/BPI_Interact.BPI_Interact_C")
          (bind _output_get (Variables|Interaction|SetHit%20Interactable%20Actor (.HitActor (Collision|BreakHitResult (Utilities|Array|Get(acopy) _outhits)))))
          (Class|BPIInteract|BPIFHoverInteraction(Message) _output_get true)
          (bind _interact_type (Class|BPIInteract|BPIFGetInteractType(Message) _output_get))
          (switch Utilities|FlowControl|Switch|SwitchonEnum_InteractType _interact_type)
          (else
            (bind _hit_interactable_actor (Variables|Interaction|GetHit%20Interactable%20Actor :!label _label)
              (:then
                (Class|BPIInteract|BPIFHoverInteraction(Message) _hit_interactable_actor false)
                (Variables|Interaction|SetHit%20Interactable%20Actor 0))
              (:else))))
        (else
          (goto _label))))))

(fn ConstructionScript)

(fn FunctRaycast
  (params (Cam%20Transform :type Transform%20%28by%20ref%29))
  (bind (_location _rotation) (Math|Transform|BreakTransform Cam%20Transform))
  (bind _outhits (Collision|MultiSphereTraceByChannel _location (+ _location (* (Math|Rotator|GetRotationXVector _rotation) 3e+02)) 1.0 "TraceTypeQuery1" false 0 "ForOneFrame"))
  (return _outhits))

(fn FunctManageinVehicleStatus
  (params (Current%20Vehicle :type Vehicle%20Base%20Object%20Reference) (inVehicle :type Boolean))
  (Variables|Vehicle|SetCurrent%20Vehicle Current%20Vehicle)
  (bind _output_get (Variables|Vehicle|SetinVehicle inVehicle))
  (if _output_get
    (Collision|SetActorEnableCollision false)
    (Transformation|AttachActorToActor (Variables|Vehicle|GetCurrent%20Vehicle) "None" "KeepRelative" "KeepRelative" "KeepRelative" false)
    (else
      (Collision|SetActorEnableCollision true)
      (Transformation|DetachFromActor "KeepRelative" "KeepRelative" "KeepRelative"))))
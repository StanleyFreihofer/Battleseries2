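; Base player soldier character that handles on-foot movement, interaction and weapons, and doubles as the input hub while seated in vehicles.
; Each tick on foot, a short sphere trace from the camera sets the hovered BPI_Interact actor for press or timed-hold interaction.
; In vehicles, Enhanced Input forwards driving, seat, horn, turret and weapon actions by seat index, and look input becomes animated head freelook.
; Raw-key debug hooks tune projectiles and print state.
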(event Custom|Interact
  ;[0.15 0.15 0.15 0.5] Interaction
  (Class|BPIInteract|BPIInteract(Message) (Variables|Default|GetHit%20Interactable%20Actor) self))

(event Custom|Complete%20Interact%20Hold
  ;[0.15 0.15 0.15 0.5] Interaction
  (CallFunction|Interact))

(event Custom|CustomEvent
  (params (UserId :type Platform%20User%20Id%20Structure) (DeviceId :type Input%20Device%20Id%20Structure))
  (Development|PrintString (Utilities|String|ToString(Integer) UserId)))

(event Custom|Start%20Interact
  ;[0.15 0.15 0.15 0.5] Interaction
  (bind _hit_interactable_actor (Variables|Default|GetHit%20Interactable%20Actor)
    (:then
      (bind _interact_type (Class|BPIInteract|BPIFGetInteractType(Message) _hit_interactable_actor))
      (switch Utilities|FlowControl|Switch|SwitchonEnum_InteractType _interact_type
        (:NewEnumerator0
          (CallFunction|Interact))
        (:NewEnumerator1
          (Utilities|FlowControl|DoOnce false
            (:Completed
              (bind _returnvalue (Utilities|Time|SetTimerbyEvent (delegate Custom|Complete%20Interact%20Hold) 1.0))
              (Variables|Default|SetTimer_Interact _returnvalue))))))
    (:else)))

(event Custom|Unequip%20Weapon)

(event Custom|Equip%20Weapon)

(event Custom|Switch%20Weapon
  (params (Weapon%20Index :type Integer))
  (Utilities|IsValid (Variables|Default|GetCurrent%20Weapon)))

(event Custom|Drop%20Weapon)

(event Custom|Stop%20Interact
  ;[0.15 0.15 0.15 0.5] Interaction
  (Utilities|Time|ClearandInvalidateTimerbyHandle (Variables|Default|GetTimer_Interact))
  (Utilities|FlowControl|DoOnce false) ; enters at Reset
)

(event Input|EnhancedActionEvents|EnhancedInputActionIA_Move
  (params (ActionValue :type Vector%202D%20Structure) (ElapsedSeconds :type Float%20%28double-precision%29) (TriggeredSeconds :type Float%20%28double-precision%29) (InputAction :type Input%20Action%20Object%20Reference :default "/Game/__SFContent/Inputs/Actions/Default/IA_Move.IA_Move"))
  (Pawn|Input|AddMovementInput (Transformation|GetActorForwardVector) (.y ActionValue) false)
  (Pawn|Input|AddMovementInput (Transformation|GetActorRightVector) (.x ActionValue) false))

(event Input|EnhancedActionEvents|EnhancedInputActionIA_Look
  (params (ActionValue :type Vector%202D%20Structure) (ElapsedSeconds :type Float%20%28double-precision%29) (TriggeredSeconds :type Float%20%28double-precision%29) (InputAction :type Input%20Action%20Object%20Reference :default "/Game/__SFContent/Inputs/Actions/Default/IA_Look.IA_Look"))
  (bind _characterstate (Variables|Default|GetCharacterState))
  (bind _charactervehiclestate (Utilities|Struct|BreakCharacterState _characterstate))
  (bind _invehicle (Utilities|Struct|BreakCharacterVehicleState _charactervehiclestate))
  (:Triggered
    (if _invehicle
      (CallFunction|Freelook true (Math|Vector2D|MakeVector2D (.x ActionValue) (.y ActionValue)))
      (else
        (Pawn|Input|AddControllerYawInput (.x ActionValue))
        (Pawn|Input|AddControllerPitchInput (.y ActionValue)))))
  (:Completed
    (if _invehicle
      _)))

(event Input|EnhancedActionEvents|EnhancedInputActionIA_Shoot
  (params (ActionValue :type Boolean) (ElapsedSeconds :type Float%20%28double-precision%29) (TriggeredSeconds :type Float%20%28double-precision%29) (InputAction :type Input%20Action%20Object%20Reference :default "/Game/__SFContent/Inputs/Actions/Default/IA_Shoot.IA_Shoot"))
  (bind _characterstate (Variables|Default|GetCharacterState))
  (bind _charactervehiclestate (Utilities|Struct|BreakCharacterState _characterstate))
  (bind (_invehicle _currentvehicle _csi) (Utilities|Struct|BreakCharacterVehicleState _charactervehiclestate))
  (bind _vehicleweaponlogiccomponent (Variables|/Script/Battleseries2.Vehicle_Base|GetVehicleWeaponLogicComponent _currentvehicle))
  (:Triggered
    (if _invehicle
      (Class|VehicleWeaponLogicComponent|HandleStartFire _vehicleweaponlogiccomponent _csi)))
  (:Completed
    (if _invehicle
      (Class|VehicleWeaponLogicComponent|StopFire _vehicleweaponlogiccomponent _csi))))

(event Input|EnhancedActionEvents|EnhancedInputActionIA_Interact
  (params (ActionValue :type Boolean) (ElapsedSeconds :type Float%20%28double-precision%29) (TriggeredSeconds :type Float%20%28double-precision%29) (InputAction :type Input%20Action%20Object%20Reference :default "/Game/__SFContent/Inputs/Actions/Default/IA_Interact.IA_Interact"))
  ;[0.15 0.15 0.15 0.5] Interaction
  (:Triggered
    (if (not (.inVehicle (Utilities|Struct|BreakCharacterVehicleState (.charactervehiclestate (Variables|Default|GetCharacterState)))))
      (CallFunction|StartInteract)))
  (:Completed
    (CallFunction|StopInteract)))

(event Input|EnhancedActionEvents|EnhancedInputActionIA_SwitchWeap
  (params (ActionValue :type Boolean) (ElapsedSeconds :type Float%20%28double-precision%29) (TriggeredSeconds :type Float%20%28double-precision%29) (InputAction :type Input%20Action%20Object%20Reference :default "/Game/__SFContent/Inputs/Actions/Default/IA_SwitchWeap.IA_SwitchWeap"))
  (bind _characterstate (Variables|Default|GetCharacterState))
  (bind _charactervehiclestate (Utilities|Struct|BreakCharacterState _characterstate))
  (bind (_invehicle _currentvehicle _csi) (Utilities|Struct|BreakCharacterVehicleState _charactervehiclestate))
  (:Started
    (if _invehicle
      (Class|VehicleWeaponLogicComponent|SwitchWeapon (Variables|/Script/Battleseries2.Vehicle_Base|GetVehicleWeaponLogicComponent _currentvehicle) _csi))))

(event EventBeginPlay
  (Utilities|FlowControl|Sequence
    (:then_0
      (bind _asbp_player_controller_base (Utilities|Casting|CastToBP_PlayerController_Base (Pawn|GetController)))
      (bind _output_get (Variables|Default|SetAs%20BP%20Player%20Controller%20Base _asbp_player_controller_base))
      (Input|AddMappingContext (PlayerController|LocalPlayerSubsystems|GetEnhancedInputLocalPlayerSubsystem _output_get) "/Game/__SFContent/Inputs/IMC/Person/IMC_Soldier.IMC_Soldier" 0 "(bIgnoreAllPressedKeysUntilRelease=True,bForceImmediately=False,bNotifyUserSettings=False)"))
    (:then_1
      (Class|HUDSubsystem|SpawnStatusHUD (Subsystems|GetHUDSubsystem (Game|GetPlayerController 0)) "/Game/__SFContent/HUD/GameplayHUDs/WB_HUD_Status.WB_HUD_Status_C"))))

(event Game|Damage|EventAnyDamage
  (params (Damage :type Float%20%28single-precision%29) (DamageType :type Damage%20Type%20Object%20Reference) (InstigatedBy :type Controller%20Object%20Reference) (DamageCauser :type Actor%20Object%20Reference))
  (Development|PrintString (Utilities|String|ToString(Float) Damage) true true "(R=1.000000,G=0.011692,B=0.000000,A=1.000000)"))

(event EventTick
  (params (DeltaSeconds :type Float%20%28single-precision%29))
  (Utilities|FlowControl|Sequence
    (:then_0
      ;[0.15 0.15 0.15 0.5] only do this if this character is possessed
      (if (and (Utilities|IsValid (Pawn|GetController)) (not (.inVehicle (Utilities|Struct|BreakCharacterVehicleState (.charactervehiclestate (Variables|Default|GetCharacterState))))))
        (bind _outhits (CallFunction|FunctRaycast (Transformation|GetWorldTransform (Variables|Default|GetCamera))))
        (if (> (Utilities|Array|Length _outhits) 0)
          (if (Utilities|DoesObjectImplementInterface (.HitActor (Collision|BreakHitResult (Utilities|Array|Get(acopy) _outhits))) "/Game/__SFContent/Generic/Utilities/Interfaces/BPI_Interact.BPI_Interact_C")
            (bind _output_get (Variables|Default|SetHit%20Interactable%20Actor (.HitActor (Collision|BreakHitResult (Utilities|Array|Get(acopy) _outhits)))))
            (Class|BPIInteract|BPIFHoverInteraction(Message) _output_get true)
            (else
              (bind _hit_interactable_actor (Variables|Default|GetHit%20Interactable%20Actor :!label _label)
                (:then
                  (Class|BPIInteract|BPIFHoverInteraction(Message) _hit_interactable_actor false)
                  (Variables|Default|SetHit%20Interactable%20Actor 0))
                (:else))))
          (else
            (goto _label)))))
    (:then_1
      (if true
        _))))

(event Input|MouseEvents|RightMouseButton
  (params (Key :type Key%20Structure :default "None"))
  (:Pressed
    (Variables|Default|SetisAiming true))
  (:Released
    (Variables|Default|SetisAiming false)))

(event Input|KeyboardEvents|T
  (params (Key :type Key%20Structure :default "None"))
  (:Pressed
    (bind _asbp_player_controller_base (Utilities|Casting|CastToBP_PlayerController_Base (Pawn|GetController)))
    (Class|PlayerControllerBase|InitCustomizationScreen _asbp_player_controller_base)))

(event Input|MouseEvents|LeftMouseButton
  (params (Key :type Key%20Structure :default "None")))

(event Input|MouseEvents|LeftMouseButton
  (params (Key :type Key%20Structure :default "None"))
  (:Pressed
    (bind _current_weapon (Variables|Default|GetCurrent%20Weapon)
      (:then
        (Default|Fire _current_weapon))
      (:else))))

(event Input|KeyboardEvents|Up
  (params (Key :type Key%20Structure :default "None"))
  (:Pressed
    (Default|ChangeDrop (Variables|Default|GetCurrent%20Weapon) 2e+01)))

(event Input|KeyboardEvents|R
  (params (Key :type Key%20Structure :default "None"))
  (bind _current_weapon (Variables|Default|GetCurrent%20Weapon))
  (bind _projectiles (Variables|/Game/__SFContent/Weapons/BP/BP_Weapon_Base.BP_Weapon_Base_C|GetProjectiles _current_weapon))
  (:Pressed
    (for _index (range 0 (Utilities|Array|Length _projectiles))
      (Development|PrintString (Utilities|String|ToString(Text) (Utilities|Text|FormatText "Location = {a} 
Velocity = {b}" (Utilities|String|ToString(Vector) (.location (Utilities|Array|Get(acopy) _projectiles _index))) (Utilities|String|ToString(Vector) (.velocity (Utilities|Array|Get(acopy) _projectiles _index)))))))))

(event Input|KeyboardEvents|Down
  (params (Key :type Key%20Structure :default "None"))
  (:Pressed
    (Default|ChangeDrop (Variables|Default|GetCurrent%20Weapon) -2e+01)))

(event Input|KeyboardEvents|Left
  (params (Key :type Key%20Structure :default "None"))
  (:Pressed
    (Default|ChangeVelocity (Variables|Default|GetCurrent%20Weapon) -1e+01)))

(event Input|KeyboardEvents|Right
  (params (Key :type Key%20Structure :default "None"))
  (:Pressed
    (Default|ChangeVelocity (Variables|Default|GetCurrent%20Weapon) 1e+01)))

(event Custom|Freelook
  (params (isFreelooking :type Boolean) (Handle%20FreeLook :type Vector%202D%20Structure))
  (bind (_x _y) (Math|Vector2D|BreakVector2D Handle%20FreeLook))
  (bind _characterstate (Variables|Default|GetCharacterState))
  (bind _charactervehiclestate (Utilities|Struct|BreakCharacterState _characterstate))
  (if isFreelooking
    (Utilities|Struct|SetmembersinCharacterVehicleState _charactervehiclestate true)
    (CallFunction|FunctRotateHead _x _y)
    (else
      (Utilities|Struct|SetmembersinCharacterVehicleState _charactervehiclestate false)
      (Class|ABPICharacter|UpdateHeadRotation(Message) (Components|SkeletalMesh|GetAnimInstance (Variables|Character|GetMesh)) "0, 0, 0")
      (Variables|Default|SetHead%20Horizontal%20Delta 0.0)
      (Variables|Default|SetHead%20Vertical%20Delta 0.0))))

(event Input|EnhancedActionEvents|EnhancedInputActionIA_Throttle
  (params (ActionValue :type Float%20%28double-precision%29) (ElapsedSeconds :type Float%20%28double-precision%29) (TriggeredSeconds :type Float%20%28double-precision%29) (InputAction :type Input%20Action%20Object%20Reference :default "/Game/__SFContent/Inputs/Actions/Vehicle/Driver/IA_Throttle.IA_Throttle"))
  (bind _returnvalue (Class|CharacterBase|GetCSI))
  (bind _characterstate (Variables|Default|GetCharacterState))
  (bind _charactervehiclestate (Utilities|Struct|BreakCharacterState _characterstate))
  (bind _currentvehicle (Utilities|Struct|BreakCharacterVehicleState _charactervehiclestate))
  (:Triggered
    (Class|VehicleBase|HandleThrottle _currentvehicle ActionValue _returnvalue))
  (:Completed
    (Class|VehicleBase|HandleThrottle _currentvehicle ActionValue _returnvalue)))

(event Input|EnhancedActionEvents|EnhancedInputActionIA_Freelook
  (params (ActionValue :type Vector%202D%20Structure) (ElapsedSeconds :type Float%20%28double-precision%29) (TriggeredSeconds :type Float%20%28double-precision%29) (InputAction :type Input%20Action%20Object%20Reference :default "/Game/__SFContent/Inputs/Actions/Vehicle/IA_Freelook.IA_Freelook"))
  (CallFunction|Freelook true ActionValue))

(event Input|EnhancedActionEvents|EnhancedInputActionIA_ChangeSeat
  (params (ActionValue :type Boolean) (ElapsedSeconds :type Float%20%28double-precision%29) (TriggeredSeconds :type Float%20%28double-precision%29) (InputAction :type Input%20Action%20Object%20Reference :default "/Game/__SFContent/Inputs/Actions/Vehicle/IA_ChangeSeat.IA_ChangeSeat"))
  (bind _characterstate (Variables|Default|GetCharacterState))
  (bind _charactervehiclestate (Utilities|Struct|BreakCharacterState _characterstate))
  (bind (_invehicle _currentvehicle) (Utilities|Struct|BreakCharacterVehicleState _charactervehiclestate))
  (:Started
    (if _invehicle
      (Class|VehicleBase|ChangeSeat _currentvehicle self))))

(event Input|EnhancedActionEvents|EnhancedInputActionIA_ControlTurret
  (params (ActionValue :type Vector%202D%20Structure) (ElapsedSeconds :type Float%20%28double-precision%29) (TriggeredSeconds :type Float%20%28double-precision%29) (InputAction :type Input%20Action%20Object%20Reference :default "/Game/__SFContent/Inputs/Actions/Vehicle/Gunner/IA_ControlTurret.IA_ControlTurret"))
  (bind _characterstate (Variables|Default|GetCharacterState))
  (bind _charactervehiclestate (Utilities|Struct|BreakCharacterState _characterstate))
  (bind (_invehicle _currentvehicle _vehiclehud _isfreelooking _csi) (Utilities|Struct|BreakCharacterVehicleState _charactervehiclestate))
  (if _invehicle
    (Class|VehicleWeaponLogicComponent|ControlTurret (Variables|/Script/Battleseries2.Vehicle_Base|GetVehicleWeaponLogicComponent _currentvehicle) ActionValue _csi)))

(event Input|EnhancedActionEvents|EnhancedInputActionIA_GV_Steering
  (params (ActionValue :type Float%20%28double-precision%29) (ElapsedSeconds :type Float%20%28double-precision%29) (TriggeredSeconds :type Float%20%28double-precision%29) (InputAction :type Input%20Action%20Object%20Reference :default "/Game/__SFContent/Inputs/Actions/Vehicle/Driver/GV/IA_GV_Steering.IA_GV_Steering"))
  (bind _returnvalue (Class|CharacterBase|GetCSI))
  (bind _characterstate (Variables|Default|GetCharacterState))
  (bind _charactervehiclestate (Utilities|Struct|BreakCharacterState _characterstate))
  (bind _currentvehicle (Utilities|Struct|BreakCharacterVehicleState _charactervehiclestate))
  (:Triggered
    (Class|VehicleBase|ApplySteeringGV _currentvehicle ActionValue _returnvalue))
  (:Completed
    (Class|VehicleBase|ApplySteeringGV _currentvehicle ActionValue _returnvalue)))

(event Input|EnhancedActionEvents|EnhancedInputActionIA_ExitVehicle
  (params (ActionValue :type Boolean) (ElapsedSeconds :type Float%20%28double-precision%29) (TriggeredSeconds :type Float%20%28double-precision%29) (InputAction :type Input%20Action%20Object%20Reference :default "/Game/__SFContent/Inputs/Actions/Vehicle/IA_ExitVehicle.IA_ExitVehicle"))
  (Class|CharacterBase|CharacterExitVehicle))

(event Input|EnhancedActionEvents|EnhancedInputActionIA_Horn
  (params (ActionValue :type Boolean) (ElapsedSeconds :type Float%20%28double-precision%29) (TriggeredSeconds :type Float%20%28double-precision%29) (InputAction :type Input%20Action%20Object%20Reference :default "/Game/__SFContent/Inputs/Actions/Vehicle/Driver/IA_Horn.IA_Horn"))
  (bind _characterstate (Variables|Default|GetCharacterState))
  (bind _charactervehiclestate (Utilities|Struct|BreakCharacterState _characterstate))
  (bind (_invehicle _currentvehicle _vehiclehud _isfreelooking _csi) (Utilities|Struct|BreakCharacterVehicleState _charactervehiclestate))
  (:Started
    (if _invehicle
      (Class|VehicleBase|PlayHorn _currentvehicle)))
  (:Completed
    (Class|VehicleBase|StopHorn _currentvehicle)))

(event Input|KeyboardEvents|2
  (params (Key :type Key%20Structure :default "None"))
  (bind _characterstate (Variables|Default|GetCharacterState))
  (bind _charactervehiclestate (Utilities|Struct|BreakCharacterState _characterstate))
  (bind (_currentvehicle _csi) (Utilities|Struct|BreakCharacterVehicleState _charactervehiclestate))
  (:Pressed
    (Class|VehicleWeaponLogicComponent|SwitchWeapon (Variables|/Script/Battleseries2.Vehicle_Base|GetVehicleWeaponLogicComponent _currentvehicle) _csi)))

(event Input|KeyboardEvents|Y
  (params (Key :type Key%20Structure :default "None"))
  (:Pressed
    (CallFunction|DebugSeats)))

(fn ConstructionScript)

(fn FunctRaycast
  (params (Cam%20Transform :type Transform%20%28by%20ref%29))
  (bind (_start _end) (CallFunction|FunctTraceStartEnd Cam%20Transform 8e+01))
  (bind _outhits (Collision|MultiSphereTraceByChannel _start _end 1.0 "TraceTypeQuery1" false 0 "None"))
  (return _outhits))

(fn FunctTESTHud
  (params (UW%20Class :type User%20Widget%20Class%20Reference) (AddRemove :type Boolean))
  (if AddRemove
    (bind _returnvalue (UserInterface|CreateWidget UW%20Class (Game|GetPlayerController 0)))
    (bind _output_get (Variables|Default|SetTest%20UW _returnvalue))
    (UserInterface|Viewport|AddtoViewport _output_get 0)
    (else
      (Widget|RemovefromParent (Variables|Default|GetTest%20UW)))))

(fn FunctRotateHead
  (params (X%20%28Roll%29 :type Float%20%28double-precision%29) (Z%20%28Yaw%29 :type Float%20%28double-precision%29))
  (bind _result (Math|Float|NegateFloat Z%20%28Yaw%29)
    (:%20%20
      (Variables|Default|SetHead%20Horizontal%20Delta (+ (Variables|Default|GetHead%20Horizontal%20Delta) X%20%28Roll%29))
      (Variables|Default|SetHead%20Vertical%20Delta (+ (Variables|Default|GetHead%20Vertical%20Delta) _result))
      (Class|ABPICharacter|UpdateHeadRotation(Message) (Components|SkeletalMesh|GetAnimInstance (Variables|Character|GetMesh)) (Math|Rotator|MakeRotator (Variables|Default|GetHead%20Horizontal%20Delta) 0.0 (Variables|Default|GetHead%20Vertical%20Delta)))
      (return (Math|Rotator|MakeRotator (Variables|Default|GetHead%20Horizontal%20Delta) 0.0 (Variables|Default|GetHead%20Vertical%20Delta))))))

(fn FunctDebugViewTarget
  (bind _returnvalue (Game|GetPlayerController 0))
  (bind _returnvalue_2 (Pawn|GetViewTarget _returnvalue))
  (Development|PrintString (Utilities|String|ToString(Text) (Utilities|Text|FormatText "View Target = {a} 
Active Camera = {b}" _returnvalue_2 (Actor|GetComponentbyClass _returnvalue_2 "/Script/Engine.CameraComponent")))))

(fn FunctVehicleRangefinderTest
  (params (Vehicle :type Vehicle%20Base%20Object%20Reference) (CSI :type Integer))
  (bind _vehicleweaponlogiccomponent (Variables|/Script/Battleseries2.Vehicle_Base|GetVehicleWeaponLogicComponent Vehicle))
  (bind _vehicleweaponsystem (Variables|/Script/Battleseries2.VehicleWeaponLogicComponent|GetVehicleWeaponSystem _vehicleweaponlogiccomponent))
  (bind _value (Utilities|Map|Find _vehicleweaponsystem 0))
  (if (not (.bHasSpecialCam (Utilities|Struct|BreakVehicleWeaponInstanceData (.VehicleWeaponInstanceData (Utilities|Struct|BreakVehicleWeapon_Runtime (Utilities|Array|Get(acopy) (.weapons _value) (.currentweaponindex (.equippedweaponstate (.vehicleweaponsystemstate _value)))))))))
    (switch Utilities|FlowControl|Switch|SwitchonE_SeatRole (.seatrole (Utilities|Array|Get(acopy) (.Seats (Utilities|Struct|BreakVehicleData (Class|VehicleBase|GetVehicleDataBP Vehicle))) CSI))
      (:Gunner
        _)
      (:DriverGunner
        _))
    (switch Utilities|FlowControl|Switch|SwitchonE_ViewMethod "Windowed")))

(fn FunctDebugProjectilePath
  (params (Muzzle%20Location :type Vector) (Hit :type Hit%20Result%20Structure%20%28by%20ref%29) (LineColor :type Linear%20Color%20Structure))
  (bind (_bblockinghit _binitialoverlap _time _distance _location _impactpoint _normal _impactnormal _physmat _hitactor _hitcomponent _hitbonename _bonename _hititem _elementindex _faceindex _tracestart _traceend) (Collision|BreakHitResult Hit))
  (if _bblockinghit
    (Rendering|Debug|DrawDebugLine Muzzle%20Location _impactpoint LineColor 2.0 1.0)
    (else
      (Rendering|Debug|DrawDebugLine _tracestart _traceend LineColor 2.0 1.0))))

(fn FunctTraceStartEnd
  (params (InTransform :type Transform%20%28by%20ref%29) (Trace%20Distance :type Float%20%28double-precision%29))
  (bind (_location _rotation) (Math|Transform|BreakTransform InTransform))
  (return _location (+ _location (* (Math|Rotator|GetRotationXVector _rotation) Trace%20Distance))))

(fn DebugSeats
  (bind _returnvalue (Actor|GetActorOfClass "/Game/__SFContent/Vehicles/BP/BP_Vehicle_Base2.BP_Vehicle_Base2_C"))
  (for (_array_element _array_index) (.SeatStates (Utilities|Struct|BreakVehicleCurrentState (Variables|/Script/Battleseries2.Vehicle_Base|GetVehicleCurrentState _returnvalue)))
    (Development|PrintString (Utilities|String|ToString(Text) (Utilities|Text|FormatText "Seat Index = {i}             Occupied = {b}" _array_index (Utilities|Text|ToText(Boolean) (.isOccupied (Utilities|Struct|BreakSeatState _array_element))))))))